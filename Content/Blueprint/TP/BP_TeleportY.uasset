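; BP_TeleportY is a trigger box that teleports the first-person character along the Y axis.
; On overlap it keeps the character's last X and Z and takes Y from a local TP coordinate transformed to world space.
; It then calls LightWinkTP on the character with its flash state and increments NbTP if BPClosingRef has ClosedOnce set.
; A sliding wall meant to hide lighting bugs is present but never runs.
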(event `self.Box.OnComponentBeginOverlap`
  (params (OverlappedComponent :type "PrimitiveComponent Object Reference") (OtherActor :type "Actor Object Reference") (OtherComp :type "PrimitiveComponent Object Reference") (OtherBodyIndex :type Integer) (bFromSweep :type Boolean) (SweepResult :type "HitResult Structure (by ref)"))
  (bind (_tp_x _tp_y) (`KismetMathLibrary.BreakVector` (`self.TP`)))
  (bind (_returnvalue_x _returnvalue_y) (`KismetMathLibrary.BreakVector` (`KismetMathLibrary.TransformLocation` (`self.GetTransform`) (`KismetMathLibrary.Conv_DoubleToVector` _tp_y))))
  ;[1 1 1] Téléporte le joueur en un Y choisi et à sa position identique en Z et en X si celui-ci entre dans la box + incrémente le NbTP de 1
  (bind _asbp_first_person_character (cast `/Game/FirstPerson/Blueprints/BP_FirstPersonCharacter` OtherActor))
  (bind (_returnvalue_x_2 _returnvalue_y_2 _returnvalue_z) (`KismetMathLibrary.BreakVector` (`CharacterMovementComponent.GetLastUpdateLocation` (`Character.CharacterMovement` _asbp_first_person_character))))
  (`self.K2_SetActorLocation` _asbp_first_person_character (`KismetMathLibrary.MakeVector` _returnvalue_x_2 _returnvalue_y _returnvalue_z) false false)
  (`/Game/FirstPerson/Blueprints/BP_FirstPersonCharacter.Light_Wink_TP` _asbp_first_person_character (`/Game/FirstPerson/Blueprints/BP_FirstPersonCharacter.isFlashOn` _asbp_first_person_character))
  ;;[1 1 1] Un mur noir apparaît puis disparaît et translate vers le fond avant de disparaitre afin d'éviter certains bugs de lumière
  (if (`/Game/Blueprint/Doors/BP_ClosingDoor.ClosedOnce` (`self.BPClosingRef`))
    (bind _result (`/Engine/EditorBlueprintResources/StandardMacros.IncrementInt` (`self.nbTP`))
      (:`  `
        (bind _output_get (set `self.nbTP` _result))))))

(fn `UserConstructionScript`)