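; Teleport trigger actor that moves the first-person player vertically to another height once the dolls objective is finished.
; When the player character stops overlapping it, it checks the character's IsDollsFinished flag, printing it as debug text.
; If true, it keeps X and Y from the movement component's last update location and derives the new Z from TP's Z, transformed by the actor's transform.
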(event `self.ReceiveActorEndOverlap`
  (params (OtherActor :type "Actor Object Reference"))
  (bind (_tp_x _tp_y _tp_z) (`KismetMathLibrary.BreakVector` (`self.TP`)))
  (bind (_returnvalue_x _returnvalue_y _returnvalue_z) (`KismetMathLibrary.BreakVector` (`KismetMathLibrary.TransformLocation` (`self.GetTransform`) (`KismetMathLibrary.Conv_DoubleToVector` _tp_z))))
  (bind _asbp_first_person_character (cast `/Game/FirstPerson/Blueprints/BP_FirstPersonCharacter` OtherActor))
  (bind _isdollsfinished (`/Game/FirstPerson/Blueprints/BP_FirstPersonCharacter.isDollsFinished` _asbp_first_person_character))
  (`KismetSystemLibrary.PrintString` (`KismetStringLibrary.Conv_BoolToString` _isdollsfinished) true true (struct :`R` 1.0 :`B` 0.828579 :`A` 1.0))
  (if _isdollsfinished
    (`KismetSystemLibrary.PrintString` (`KismetStringLibrary.Conv_BoolToString` _isdollsfinished) true true (struct :`R` 1.0 :`B` 0.828579 :`A` 1.0))
    (bind (_returnvalue_x_2 _returnvalue_y_2) (`KismetMathLibrary.BreakVector` (`CharacterMovementComponent.GetLastUpdateLocation` (`Character.CharacterMovement` _asbp_first_person_character))))
    (`self.K2_SetActorLocation` _asbp_first_person_character (`KismetMathLibrary.MakeVector` _returnvalue_x_2 _returnvalue_y_2 _returnvalue_z) false false)))

(fn `UserConstructionScript`)