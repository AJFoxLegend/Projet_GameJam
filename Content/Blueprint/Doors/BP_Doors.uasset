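; Interactive door actor that swings its mesh open or closed in yaw.
; Separate open and close timelines lerp between RotationPos and an offset closed yaw set at BeginPlay, restarting the door sound on every update.
; Interact only opens the door, plus its twin when flagged as a portal.
; Portal spawning and linking logic is disconnected, leaving Create_TP empty.
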(event `self.ReceiveBeginPlay`
  ;[1 1 1] Mise en place des valeurs de la porte
  (set `self.closeRotPos` (- (`self.rotationPos`) 140.0)))

(event `openDoor`
  (bind _sc_porte (`self.SC_Porte`))
  ;[1 1 1] Evénement correspondant à l'ouverture de la porte
  (if (`self.isClosed`)
    (set `self.isClosed` false)
    (`KismetSystemLibrary.PrintString` "Open")
    (bind (_direction _rotationvalue) (`Timeline|Timeline_1` :!via `PlayFromStart`)
      (:`Update`
        ;;[1 1 1] CloseRotPos = La rotation de la porte fermée
        ;; Rotation Pos = La rotation de la porte ouverte
        (`SceneComponent.K2_SetWorldRotation` (`self.DoorStaticMeshComponent`) (`KismetMathLibrary.MakeRotator` 0.0 0.0 (`KismetMathLibrary.Lerp` (`self.closeRotPos`) (`self.rotationPos`) _rotationvalue)) false false)
        ;[1 1 1] Son
        (`AudioParameterControllerInterface.SetBoolParameter` _sc_porte "IsOpen" false)
        (`AudioComponent.Play` _sc_porte 0.0)))))

(event `CloseDoor`
  (bind _sc_porte (`self.SC_Porte`))
  ;[1 1 1] Evénement correspondant à la fermeture de la porte
  (if (not (`self.isClosed`))
    (set `self.isClosed` true)
    (bind (_direction _rotationvalue) (`Timeline|Closing Door` :!via `PlayFromStart`)
      (:`Update`
        ;;[1 1 1] CloseRotPos = La rotation de la porte fermée
        ;; Rotation Pos = La rotation de la porte ouverte
        (`SceneComponent.K2_SetWorldRotation` (`self.DoorStaticMeshComponent`) (`KismetMathLibrary.MakeRotator` 0.0 0.0 (`KismetMathLibrary.Lerp` (`self.rotationPos`) (`self.closeRotPos`) _rotationvalue)) false false)
        ;[1 1 1] Son
        (`AudioParameterControllerInterface.SetBoolParameter` _sc_porte "IsOpen" true)
        (`AudioComponent.Play` _sc_porte 0.0)))))

(event `/Game/FirstPerson/Blueprints/BPI_Interaction.Interact`
  ;[1 1 1] Evénement d'intéraction
  (if (`self.isInteractive`)
    (if (`self.isPortal`)
      (`self.openDoor` self)
      (`self.openDoor` (`self.Door Twin ref`))
      (else
        (`self.openDoor` self)))))

(event `Create_TP`)

(event `Destroy`
  (`/Engine/EditorBlueprintResources/StandardMacros.IsValid` (`self.Other`)
    (:`Is Valid`
      (`self.Destroy_Propre` (`self.Other`))
      (`self.Destroy_Propre` null))))

(event `Destroy_Propre`
  (params (portal :type "/Game/Portal/BP_Portal Object Reference"))
  (bind _output_get (set `self.Other` portal))
  (`self.K2_DestroyActor` _output_get))

(fn `UserConstructionScript`)