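; BP_Animation is an actor that plays a camera animation for a death sequence.
; PlayAnimationDead starts a Gameplay Cameras animation, blends the player's view to this actor, then after a short delay runs a timeline whose event calls EndAnimation.
; End_Animation returns the view to the player character, then destroys the actor after a delay.
; The branch that would stop the camera animation is unconnected and never runs.
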(event `PlayAnimationDead`
  (bind _returnvalue (`GameplayStatics.GetPlayerController` 0))
  (bind _returnvalue_2 (`GameplayCamerasSubsystem.PlayCameraAnimation` :`self` (subsystem `GameplayCamerasSubsystem`) :`PlayerController` _returnvalue :`Sequence` "/Game/Ilian/NewCameraAnimationSequence.NewCameraAnimationSequence"))
  (`PlayerController.SetViewTargetWithBlend` _returnvalue self 0.0 "VTBlend_Linear" 0.0 false)
  (`KismetSystemLibrary.Delay` 0.2)
  (`Timeline|Timeline` :!via `PlayFromStart`
    (:`he`
      (`self.End_Animation`))))

(event `End_Animation`
  (`PlayerController.SetViewTargetWithBlend` (`GameplayStatics.GetPlayerController` 0) (`GameplayStatics.GetPlayerCharacter` 0) 0.0 "VTBlend_Linear" 0.0 false)
  (`KismetSystemLibrary.Delay` 0.2)
  (`self.K2_DestroyActor`))

(fn `UserConstructionScript`)