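; BP_MasterIABT is an AI-controlled actor that feeds its perception results into a Blackboard, tracking whether the player is seen.
; On each AIPerception target update, a successful sense sets isPlayerSeen and clears hasSeenPlayer.
; A lost stimulus flips both flags and stores the stimulus location as lastSeenPlayerLocation.
; The event filters neither sensed actor nor sense type, and prints debug text for both outcomes.
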(event `self.AIPerception.OnTargetPerceptionUpdated`
  (params (Actor :type "Actor Object Reference") (Stimulus :type "AIStimulus Structure"))
  (bind _returnvalue (`AIBlueprintHelperLibrary.GetBlackboard` (`AIBlueprintHelperLibrary.GetAIController` self)))
  ;[1 1 1] Sight Perception
  (if Stimulus_bSuccessfullySensed
    (`KismetSystemLibrary.PrintString` "Seen")
    (`BlackboardComponent.SetValueAsBool` _returnvalue "isPlayerSeen" true)
    (`BlackboardComponent.SetValueAsBool` _returnvalue "hasSeenPlayer" false)
    (else
      (`KismetSystemLibrary.PrintString` "Not seen")
      (`BlackboardComponent.SetValueAsBool` _returnvalue "isPlayerSeen" false)
      (`BlackboardComponent.SetValueAsBool` _returnvalue "hasSeenPlayer" true)
      (`BlackboardComponent.SetValueAsVector` _returnvalue "lastSeenPlayerLocation" Stimulus_StimulusLocation))))

(fn `UserConstructionScript`)