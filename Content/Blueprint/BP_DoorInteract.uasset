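; Door Blueprint that swings open when its Interact event fires while it is closed.
; Interact clears IsClosed and plays the OpeningDoor timeline, whose RotationValue drives a Lerp on the mesh's world yaw toward the negated RotationAngle.
; The Lerp starts from the current yaw on each update, and pitch and roll are set to zero.
; The graph has no closing path.
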(event `/Game/FirstPerson/Blueprints/BPI_Interaction.Interact`
  (bind (_returnvalue_roll _returnvalue_pitch _returnvalue_yaw) (`KismetMathLibrary.BreakRotator` (`SceneComponent.K2_GetComponentRotation` (`self.DoorStaticMeshComponent`))))
  (if (`self.isClosed`)
    (set `self.isClosed` false)
    (bind (_direction _rotationvalue) (`Timeline|Opening Door` :!via `PlayFromStart`)
      (:`Update`
        (`SceneComponent.K2_SetWorldRotation` (`self.DoorStaticMeshComponent`) (`KismetMathLibrary.MakeRotator` 0.0 0.0 (`KismetMathLibrary.Lerp` _returnvalue_yaw (* (`self.rotationAngle`) -1.0) _rotationvalue)) false false)))))

(fn `UserConstructionScript`)