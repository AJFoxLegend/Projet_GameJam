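; BP_ScriptedDoor is a door Blueprint that swings open or closed through the openDoor and CloseDoor events, which comments tie to the Tunnel to Room 1 door.
; Each event plays its own timeline from the start, lerping the mesh's world yaw between CloseRotPos and RotationPos.
; Only CloseDoor derives CloseRotPos, as 90 degrees below RotationPos; openDoor uses the stored value as is.
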(event `openDoor`
  ;[1 1 1] Evénement correspondant à l'ouverture de la porte Tunnel -> Salle 1
  (bind (_direction _rotationvalue) (`Timeline|Opening Door` :!via `PlayFromStart`)
    (:`Update`
      ;;[1 1 1] CloseRotPos = La rotation de la porte fermée
      ;; Rotation Pos = La rotation de la porte ouverte
      (`SceneComponent.K2_SetWorldRotation` (`self.DoorStaticMeshComponent`) (`KismetMathLibrary.MakeRotator` 0.0 0.0 (`KismetMathLibrary.Lerp` (`self.closeRotPos`) (`self.rotationPos`) _rotationvalue)) false false))))

(event `CloseDoor`
  ;[1 1 1] Evénement correspondant à la fermeture de la porte Tunnel -> Salle 1
  (set `self.closeRotPos` (- (`self.rotationPos`) 90.0))
  (bind (_direction _rotationvalue) (`Timeline|Closing Door` :!via `PlayFromStart`)
    (:`Update`
      ;;[1 1 1] CloseRotPos = La rotation de la porte fermée
      ;; Rotation Pos = La rotation de la porte ouverte
      (`SceneComponent.K2_SetWorldRotation` (`self.DoorStaticMeshComponent`) (`KismetMathLibrary.MakeRotator` 0.0 0.0 (`KismetMathLibrary.Lerp` (`self.rotationPos`) (`self.closeRotPos`) _rotationvalue)) false false))))

(fn `UserConstructionScript`)