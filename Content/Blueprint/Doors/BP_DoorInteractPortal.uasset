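; BP_DoorInteractPortal is an interactable door linked to a second door and to a portal.
; Interact plays the OpeningDoor timeline, swinging both doors 90 degrees in yaw, and CloseDoor reverses it.
; The timeline update sets the portal's BoolIsActive to IsClosed: false immediately while open, true after a one-second delay when closing.
; BeginPlay starts the portal with that flag true.
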(event `self.ReceiveBeginPlay`
  (set `/Game/Portal/BP_Portal.BoolIsActive` true (`self.PortalRef`)))

(event `self.Interact`
  (bind _isclosed (`self.isClosed`))
  (bind _rotationpos (`self.rotationPos`))
  (bind _portalref (`self.PortalRef`))
  ;[1 1 1] Evénement correspondant à l'ouverture des portes avec lesquelles on peut intéragir
  (if (`self.isClosed`)
    (set `self.isClosed` false)
    (bind (_direction _rotationvalue) (`Timeline|Opening Door` :!via `PlayFromStart` :!label _label)
      (:`Update`
        ;;[1 1 1] Rotation Pos = La rotation de la porte ouverte
        (`SceneComponent.K2_SetRelativeRotation` (`self.DoorStaticMeshComponent`) (`KismetMathLibrary.MakeRotator` 0.0 0.0 (`KismetMathLibrary.Lerp` _rotationpos (+ _rotationpos 90.0) _rotationvalue)) false false)
        (`SceneComponent.K2_SetRelativeRotation` (`/Game/Blueprint/Doors/BP_DoorInteractPortal.DoorStaticMeshComponent` (`self.Door_Link`)) (`KismetMathLibrary.MakeRotator` 0.0 0.0 (`KismetMathLibrary.Lerp` _rotationpos (+ _rotationpos 90.0) _rotationvalue)) false false)
        (if _isclosed
          (`KismetSystemLibrary.Delay` 1.0)
          (set `/Game/Portal/BP_Portal.BoolIsActive` _isclosed _portalref)
          (else
            (set `/Game/Portal/BP_Portal.BoolIsActive` _isclosed _portalref)))))))

(event `CloseDoor`
  ;[1 1 1] Evénement correspondant à l'ouverture des portes avec lesquelles on peut intéragir
  (if (not (`self.isClosed`))
    (set `self.isClosed` true)
    (goto _label :!via `ReverseFromEnd`)))

(fn `UserConstructionScript`)