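; Trigger box actor that scripts a tunnel door's closing and reopening as the first-person character passes through.
; Entering closes the door if it is interactive or on the first pass.
; After two infinite-tunnel teleports, later entries reopen it, or, for rooms, close it and destroy the trigger.
; Once four voodoo dolls are placed, exiting, or entering after reopening, closes the door and makes it interactive.
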(event `self.Box.OnComponentBeginOverlap`
  (params (OverlappedComponent :type "PrimitiveComponent Object Reference") (OtherActor :type "Actor Object Reference") (OtherComp :type "PrimitiveComponent Object Reference") (OtherBodyIndex :type Integer) (bFromSweep :type Boolean) (SweepResult :type "HitResult Structure (by ref)"))
  ;[1 1 1] Script Porte tunnel qui se ferme
  ;;[1 1 1] Si on entre dans la box alors on vérifie si la porte est intéractive
  (cast `/Game/FirstPerson/Blueprints/BP_FirstPersonCharacter` OtherActor)
  (if (`/Game/Blueprint/Doors/BP_Doors.isInteractive` (`self.BPDoorRef`))
    ;;[1 1 1] Si c'est le cas, entré dans la box ferme la porte
    (`/Game/Blueprint/Doors/BP_Doors.closeDoor` (`self.BPDoorRef`))
    (`KismetSystemLibrary.PrintString` "Close")
    (else
      ;;[1 1 1] On regarde si la porte s'est déja fermée une première fois
      (if (`self.ClosedOnce`)
        ;;[1 1 1] Si la porte est fermée, alors on vérifie si l'on a pris le tunnel infini au moins deux fois, si c'est le cas, alors la porte s'ouvre et le booléen "ReOpen" passe en True
        (if (>= (`/Game/Blueprint/TP/BP_TP.nbTP` (`self.tpRef`)) 2)
          ;;;[1 1 1] Si l'on pénètre dans la chambre, la porte se ferme, sinon, elle reste ouverte
          (if (`self.isRoom`)
            (`/Game/Blueprint/Doors/BP_Doors.CloseDoor` (`self.BPDoorRef`))
            (`KismetSystemLibrary.PrintString` "Close")
            (`KismetSystemLibrary.Delay` 0.5)
            (`self.K2_DestroyActor`)
            (elif (`self.ReOpen`)
              ;;[1 1 1] Si la quête des voodoo dolls a été terminée alors, la porte se ferme et devient intéractive
              (if (>= (`/Game/Blueprint/VoodooDolls/BP_Inventory.nbPuttingDolls` (`self.InventoryRef`)) 4) :!label _label
                (`/Game/Blueprint/Doors/BP_Doors.closeDoor` (`self.BPDoorRef`))
                (set `/Game/Blueprint/Doors/BP_Doors.isInteractive` true (`self.BPDoorRef`))
                (`KismetSystemLibrary.PrintString` "is Interactive" true true (struct :`R` 1.0 :`B` 0.053995 :`A` 1.0)))
              (else
                (`KismetSystemLibrary.PrintString` "Open")
                (`/Game/Blueprint/Doors/BP_Doors.openDoor` (`self.BPDoorRef`))
                (set `self.ReOpen` true)))))
        (else
          ;;[1 1 1] Si la porte n'est pas fermée, alors on la ferme en appelant l'event Close Door et on passe en true le booléen "Closed Once"
          (`KismetSystemLibrary.PrintString` "Close")
          (`/Game/Blueprint/Doors/BP_Doors.closeDoor` (`self.BPDoorRef`))
          (set `self.ClosedOnce` true))))))

(event `self.Box.OnComponentEndOverlap`
  (params (OverlappedComponent :type "PrimitiveComponent Object Reference") (OtherActor :type "Actor Object Reference") (OtherComp :type "PrimitiveComponent Object Reference") (OtherBodyIndex :type Integer))
  ;[1 1 1] Script Porte tunnel qui se ferme
  ;;[1 1 1] Si on entre dans la box alors on vérifie si la porte est intéractive
  (cast `/Game/FirstPerson/Blueprints/BP_FirstPersonCharacter` OtherActor)
  (goto _label))

(fn `UserConstructionScript`)