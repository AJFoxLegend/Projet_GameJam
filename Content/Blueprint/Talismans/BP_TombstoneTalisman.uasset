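; BP_TombstoneTalisman is an interactable tombstone that accepts one talisman as part of a three-talisman door puzzle.
; Interact checks the referenced inventory's carried count and its own placed flag, printing a message when placement is not possible.
; On placement it moves one talisman from carried to placed in the inventory and spawns a scaled-down BP_TalismanOnTombstone above itself.
; Once three are placed, it opens the referenced door after a short delay.
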(event `self.Interact`
  (bind _returnvalue (`self.GetTransform`))
  ;[1 1 1] Evénement qui récupère les poupées dans la salle puis les pose sur l'autel
  ;;[1 1 1] Si l'on possède moins de 1 talisman alors rien ne se passe et un texte nous dit que nous n'avons aucun talisman
  (if (> (`/Game/Blueprint/VoodooDolls/BP_Inventory.nbKeepingTalisman` (`self.InventoryRef`)) 0)
    (if (`self.isTalismanPut`)
      (`KismetSystemLibrary.PrintString` "Youalready put the good talisman on this tombstone" true true (struct :`R` 1.0 :`B` 0.050213 :`A` 1.0))
      (else
        ;;[1 1 1] Si l'on possède 1 ou plusieurs talismans, alors la fois où on intéragit avec la tombe, un talisman nous est enlevée du "nbKeepingTalismans"
        (bind _result (`/Engine/EditorBlueprintResources/StandardMacros.DecrementInt` (`/Game/Blueprint/VoodooDolls/BP_Inventory.nbKeepingTalisman` (`self.InventoryRef`)))
          (:`  `
            (bind _output_get (set `/Game/Blueprint/VoodooDolls/BP_Inventory.nbKeepingTalisman` _result (`self.InventoryRef`)))
            (`KismetSystemLibrary.PrintString` (`KismetStringLibrary.Conv_IntToString` _output_get) true true (struct :`R` 1.0 :`B` 0.011788 :`A` 1.0))
            ;;[1 1 1] On vérifie que le talisman est bien posé, il voit sa visibilité être activée, permettant une sensation d'être posé sur la tombe
            (bind _output_get_2 (set `self.isTalismanPut` true))
            (`KismetSystemLibrary.PrintString` (`KismetStringLibrary.Conv_BoolToString` _output_get_2) true true (struct :`G` 1.0 :`B` 0.006993 :`A` 1.0))
            (bind _output_get_3 (set `self.talismanLoc` (`KismetMathLibrary.MakeVector` (.x (.location _returnvalue)) (.y (.location _returnvalue)) (+ (.z (.location _returnvalue)) 37.0))))
            (`|SpawnActorFromClass` "/Game/Blueprint/Talismans/BP_TalismanOnTombstone.BP_TalismanOnTombstone_C" (`KismetMathLibrary.MakeTransform` _output_get_3 (.rotation _returnvalue) (0.5 0.5 0.5)) "AdjustIfPossibleButAlwaysSpawn" "MultiplyWithRoot" null null)
            ;;[1 1 1] On incrémente le "nbPuttingTalisman" de l'inventory
            (bind _result_2 (`/Engine/EditorBlueprintResources/StandardMacros.IncrementInt` (`/Game/Blueprint/VoodooDolls/BP_Inventory.nbPuttingTalisman` (`self.InventoryRef`)))
              (:`  `
                (bind _output_get_4 (set `/Game/Blueprint/VoodooDolls/BP_Inventory.nbPuttingTalisman` _result_2 (`self.InventoryRef`)))
                ;;[1 1 1] Si les 3 talismans sont posées sur les pierres tombales, alors la porte s'ouvre
                (if (>= _output_get_4 3)
                  (`KismetSystemLibrary.Delay` 1.0)
                  (`/Game/Blueprint/Doors/BP_Doors.openDoor` (`self.DoorRef`)))))))))
    (else
      (`KismetSystemLibrary.PrintString` "You don't have any talisman" true true (struct :`R` 1.0 :`B` 0.050213 :`A` 1.0)))))

(fn `UserConstructionScript`)