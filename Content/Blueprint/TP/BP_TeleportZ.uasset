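; BP_TeleportZ is a trigger actor that teleports the player vertically once all four dolls have been placed and the player leaves its overlap.
; On ActorEndOverlap with BP_FirstPersonCharacter, it checks that the inventory reference counts four placed dolls.
; It keeps X and Y from the movement component's last update location and derives the new Z from the TP variable, transformed from the actor's local space.
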(event `self.ReceiveActorEndOverlap`
  (params (OtherActor :type "Actor Object Reference"))
  (bind (_tp_x _tp_y _tp_z) (`KismetMathLibrary.BreakVector` (`self.TP`)))
  (bind (_returnvalue_x _returnvalue_y _returnvalue_z) (`KismetMathLibrary.BreakVector` (`KismetMathLibrary.TransformLocation` (`self.GetTransform`) (`KismetMathLibrary.Conv_DoubleToVector` _tp_z))))
  ;[1 1 1] Si les 4 poupées ont été posées et que le joueur sort de la box, alors Téléporte le joueur en un Z choisi et à sa position identique en X et en Y si celui-ci sort de la box
  (bind _asbp_first_person_character (cast `/Game/FirstPerson/Blueprints/BP_FirstPersonCharacter` OtherActor))
  (if (== (`/Game/Blueprint/VoodooDolls/BP_Inventory.nbPuttingDolls` (`self.InventoryRef`)) 4)
    (bind (_returnvalue_x_2 _returnvalue_y_2) (`KismetMathLibrary.BreakVector` (`CharacterMovementComponent.GetLastUpdateLocation` (`Character.CharacterMovement` _asbp_first_person_character))))
    (`self.K2_SetActorLocation` _asbp_first_person_character (`KismetMathLibrary.MakeVector` _returnvalue_x_2 _returnvalue_y_2 _returnvalue_z) false false)))

(fn `UserConstructionScript`)