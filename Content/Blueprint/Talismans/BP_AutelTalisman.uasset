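; Talisman altar that the player interacts with to place carried talismans and open the Sakura door.
; BeginPlay hides four placed-talisman cubes unless the inventory's NbPuttingDolls count is already at least four.
; Each Interact moves one talisman from the inventory's kept count to its placed count, revealing cubes cumulatively, or prints a warning if none are held.
; At three placed, the door opens after a short delay; the fourth cube is never revealed here.
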(event `self.ReceiveBeginPlay`
  ;[1 1 1] Met chaque poupée Vaudou sur l'autel en visibilité nulle dès le commencement
  (if (not (>= (`/Game/Blueprint/VoodooDolls/BP_Inventory.nbPuttingDolls` (`self.InventoryRef`)) 4))
    (`SceneComponent.SetVisibility` (`/Game/Blueprint/VoodooDolls/BP_VoodooDollsOnAutel.Cube` (`self.TalismanRef2`)) false false)
    (`SceneComponent.SetVisibility` (`/Game/Blueprint/VoodooDolls/BP_VoodooDollsOnAutel.Cube` (`self.TalismanRef3`)) false false)
    (`SceneComponent.SetVisibility` (`/Game/Blueprint/VoodooDolls/BP_VoodooDollsOnAutel.Cube` (`self.TalismanRef4`)) false false)
    (`SceneComponent.SetVisibility` (`/Game/Blueprint/VoodooDolls/BP_VoodooDollsOnAutel.Cube` (`self.TalismanRef5`)) false false)))

(event `self.Interact`
  ;[1 1 1] Evénement qui récupère les poupées dans la salle puis les pose sur l'autel
  ;;[1 1 1] Si l'on possède moins de 1 talisman alors rien ne se passe et un texte nous dit que nous n'avons aucun talisman
  (if (> (`/Game/Blueprint/VoodooDolls/BP_Inventory.nbKeepingTalisman` (`self.InventoryRef`)) 0)
    ;;;[1 1 1] Si l'on possède 1 ou plusieurs talismans, alors à chaque fois qu'on intéragit avec l'autel, une poupée nous est enlevée du "nbKeepingTalismans"
    (bind _result (`/Engine/EditorBlueprintResources/StandardMacros.DecrementInt` (`/Game/Blueprint/VoodooDolls/BP_Inventory.nbKeepingTalisman` (`self.InventoryRef`)))
      (:`  `
        (bind _output_get (set `/Game/Blueprint/VoodooDolls/BP_Inventory.nbKeepingTalisman` _result (`self.InventoryRef`)))
        (`KismetSystemLibrary.PrintString` (`KismetStringLibrary.Conv_IntToString` _output_get) true true (struct :`R` 1.0 :`B` 0.011788 :`A` 1.0))
        ;;[1 1 1] Pour chaque talisman posée sur l'autel, cela incrémente de 1 la variable "NbPuttingTalismans",
        (bind _result_2 (`/Engine/EditorBlueprintResources/StandardMacros.IncrementInt` (`/Game/Blueprint/VoodooDolls/BP_Inventory.nbPuttingTalisman` (`self.InventoryRef`)))
          (:`  `
            (bind _output_get_2 (set `/Game/Blueprint/VoodooDolls/BP_Inventory.nbPuttingTalisman` _result_2 (`self.InventoryRef`)))
            (`KismetSystemLibrary.PrintString` (`KismetStringLibrary.Conv_IntToString` _output_get_2) true true (struct :`G` 1.0 :`B` 0.006993 :`A` 1.0))
            ;;[1 1 1] Pour chaque talisman posé sur l'autel, chacun des talismans voit sa visibilité être activée, permettant une sensation d'être posé sur l'autel
            (if (>= (`/Game/Blueprint/VoodooDolls/BP_Inventory.nbPuttingTalisman` (`self.InventoryRef`)) 1)
              (`SceneComponent.SetVisibility` (`/Game/Blueprint/VoodooDolls/BP_VoodooDollsOnAutel.Cube` (`self.TalismanRef2`)) true false)
              (if (>= (`/Game/Blueprint/VoodooDolls/BP_Inventory.nbPuttingTalisman` (`self.InventoryRef`)) 2)
                (`SceneComponent.SetVisibility` (`/Game/Blueprint/VoodooDolls/BP_VoodooDollsOnAutel.Cube` (`self.TalismanRef3`)) true false)
                (if (>= (`/Game/Blueprint/VoodooDolls/BP_Inventory.nbPuttingTalisman` (`self.InventoryRef`)) 3)
                  (`SceneComponent.SetVisibility` (`/Game/Blueprint/VoodooDolls/BP_VoodooDollsOnAutel.Cube` (`self.TalismanRef4`)) true false)
                  ;;[1 1 1] Si les 4 poupées sont posées sur l'autel, alors la porte s'ouvre
                  (`KismetSystemLibrary.Delay` 1.0)
                  (`/Game/Blueprint/Doors/BP_ScriptedDoor.openDoor` (`self.BPSakuraDoorRef`)))))))))
    (else
      (`KismetSystemLibrary.PrintString` "You don't have any talisman" true true (struct :`R` 1.0 :`B` 0.050213 :`A` 1.0)))))

(fn `UserConstructionScript`)