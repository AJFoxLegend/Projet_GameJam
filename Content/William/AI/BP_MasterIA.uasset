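; Master AI character that chases, searches for and patrols around the player, driven by AI Perception events and AIMoveTo rather than a behavior tree.
; Sighting a target starts a chase; losing it sends the pawn to the last stimulus location.
; Unless the player is seen again, it probes random navmesh points in a widening radius with random pauses.
; After those attempts it resets and loops random patrol moves around its current position.
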(event `self.AIPerception.OnTargetPerceptionUpdated`
  (params (Actor :type "Actor Object Reference") (Stimulus :type "AIStimulus Structure"))
  (if Stimulus_bSuccessfullySensed
    (`KismetSystemLibrary.PrintString` "Seen")
    (set `self.IsPlayerSeen` true)
    (`self.GoToPlayer` Actor)
    (else
      (`KismetSystemLibrary.PrintString` "Not seen")
      (set `self.IsPlayerSeen` false)
      (`self.SearchForPlayer` Stimulus_StimulusLocation))))

(event `GoToPlayer`
  (params (TargetActor :type "Actor Object Reference"))
  (`KismetSystemLibrary.PrintString` "GoToPlayer" true true (struct :`R` 1.0 :`B` 0.035882 :`A` 1.0))
  (`MovementComponent.StopMovementImmediately` (`self.CharacterMovement`))
  (`|AIMoveTo` self (0.0 0.0 0.0) TargetActor
    (:`OnSuccess`
      _)
    (:`OnFail`
      _))
  (if (`self.IsPlayerSeen`)
    (`KismetSystemLibrary.PrintString` "Behind You" true true (struct :`R` 1.0 :`G` 0.90957 :`A` 1.0))))

(event `SearchForPlayer`
  (params (LastSeenLocation :type "Vector Structure"))
  (`KismetSystemLibrary.PrintString` "SearchForPlayer" true true (struct :`R` 1.0 :`B` 0.071934 :`A` 1.0))
  (set `self.LocToSearchForPlayer` LastSeenLocation)
  (`MovementComponent.StopMovementImmediately` (`self.CharacterMovement`))
  (`|AIMoveTo` self (`self.LocToSearchForPlayer`) null 5.0 true
    (:`OnSuccess`
      _)
    (:`OnFail`
      _))
  (`KismetSystemLibrary.Delay` (`KismetMathLibrary.RandomFloatInRange` 1.0 3.0))
  (if (`self.IsPlayerSeen`)
    (`self.GoToPlayer` (`GameplayStatics.GetPlayerCharacter` 0))
    (else
      (if (< (`self.i`) 3) :!label _label
        (`/Engine/EditorBlueprintResources/StandardMacros.IncrementInt` (`self.i`)
          (:`  `
            (bind _randomlocation (`NavigationSystemV1.K2_GetRandomLocationInNavigableRadius` (`self.LocToSearchForPlayer`) (`self.RadiusToSearchPlayer`) null null))
            (bind _output_get (set `self.LocToSearchForPlayer` _randomlocation))
            (set `self.RadiusToSearchPlayer` (* (`self.RadiusToSearchPlayer`) 1.5))
            (`|AIMoveTo` self _output_get null
              (:`OnSuccess`
                _)
              (:`OnFail`
                _))
            (`KismetSystemLibrary.Delay` (`KismetMathLibrary.RandomFloatInRange` 1.0 3.0))
            (goto _label)))
        (else
          (set `self.i` 0)
          (set `self.RadiusToSearchPlayer` 500.0)
          (`self.ReturnToPatrol`))))))

(event `ReturnToPatrol`
  (`MovementComponent.StopMovementImmediately` (`self.CharacterMovement`) :!label _label_2)
  (bind _randomlocation (`NavigationSystemV1.K2_GetRandomLocationInNavigableRadius` (`self.K2_GetActorLocation`) 750.0 null null))
  (`|AIMoveTo` self _randomlocation null 3.0
    (:`OnSuccess`
      _)
    (:`OnFail`
      _))
  (`KismetSystemLibrary.Delay` 5.0)
  (goto _label_2))

(fn `UserConstructionScript`)