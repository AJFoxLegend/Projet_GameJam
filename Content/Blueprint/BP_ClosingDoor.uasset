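; BP_ClosingDoor is a trigger that closes a referenced door behind an overlap and can later reopen it.
; The first Box overlap closes the door and latches a closed flag.
; Later overlaps open it once, only if the referenced BPTP reports an NbTP count of exactly two.
; Overlaps are not filtered by actor, and both actions print debug strings.
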(event `self.Box.OnComponentBeginOverlap`
  (params (OverlappedComponent :type "PrimitiveComponent Object Reference") (OtherActor :type "Actor Object Reference") (OtherComp :type "PrimitiveComponent Object Reference") (OtherBodyIndex :type Integer) (bFromSweep :type Boolean) (SweepResult :type "HitResult Structure (by ref)"))
  (if (`self.ClosedOnce`)
    (if (and (== (`/Game/Blueprint/BP_TeleportTunnel.nbTP` (`self.BPTP`)) 2) (not (`self.ReOpen`)))
      (`KismetSystemLibrary.PrintString` "Open")
      (`/Game/Blueprint/BP_Door.openDoor` (`self.BPDoorRef`))
      (set `self.ReOpen` true))
    (else
      (`KismetSystemLibrary.PrintString` "Close")
      (`/Game/Blueprint/BP_Door.closeDoor` (`self.BPDoorRef`))
      (set `self.ClosedOnce` true))))

(fn `UserConstructionScript`)