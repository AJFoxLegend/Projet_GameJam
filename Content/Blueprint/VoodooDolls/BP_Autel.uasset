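; Altar actor where the player deposits carried voodoo dolls to open a door.
; On BeginPlay it hides four referenced doll meshes.
; Each Interact moves one doll from the inventory's carried count to its placed count, printing both, and reveals meshes up to the placed total.
; With four placed, it waits a second and calls OpenDoor on the door; with none carried, it prints a warning.
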(event `self.ReceiveBeginPlay`
  (`SceneComponent.SetVisibility` (`/Game/Blueprint/VoodooDolls/BP_VoodooDollsOnAutel.Cube` (`self.DollsRef2`)) false false)
  (`SceneComponent.SetVisibility` (`/Game/Blueprint/VoodooDolls/BP_VoodooDollsOnAutel.Cube` (`self.DollsRef3`)) false false)
  (`SceneComponent.SetVisibility` (`/Game/Blueprint/VoodooDolls/BP_VoodooDollsOnAutel.Cube` (`self.DollsRef4`)) false false)
  (`SceneComponent.SetVisibility` (`/Game/Blueprint/VoodooDolls/BP_VoodooDollsOnAutel.Cube` (`self.DollsRef5`)) false false))

(event `/Game/FirstPerson/Blueprints/BPI_Interaction.Interact`
  (if (> (`/Game/Blueprint/VoodooDolls/BP_Inventory.nbKeepigDolls` (`self.InventoryRef`)) 0)
    (bind _result (`/Engine/EditorBlueprintResources/StandardMacros.DecrementInt` (`/Game/Blueprint/VoodooDolls/BP_Inventory.nbKeepigDolls` (`self.InventoryRef`)))
      (:`  `
        (bind _output_get (set `/Game/Blueprint/VoodooDolls/BP_Inventory.nbKeepigDolls` _result (`self.InventoryRef`)))
        (`KismetSystemLibrary.PrintString` (`KismetStringLibrary.Conv_IntToString` _output_get) true true (struct :`R` 1.0 :`B` 0.011788 :`A` 1.0))
        (bind _result_2 (`/Engine/EditorBlueprintResources/StandardMacros.IncrementInt` (`/Game/Blueprint/VoodooDolls/BP_Inventory.nbPuttingDolls` (`self.InventoryRef`)))
          (:`  `
            (bind _output_get_2 (set `/Game/Blueprint/VoodooDolls/BP_Inventory.nbPuttingDolls` _result_2 (`self.InventoryRef`)))
            (`KismetSystemLibrary.PrintString` (`KismetStringLibrary.Conv_IntToString` _output_get_2) true true (struct :`G` 1.0 :`B` 0.006993 :`A` 1.0))
            (if (>= (`/Game/Blueprint/VoodooDolls/BP_Inventory.nbPuttingDolls` (`self.InventoryRef`)) 1)
              (`SceneComponent.SetVisibility` (`/Game/Blueprint/VoodooDolls/BP_VoodooDollsOnAutel.Cube` (`self.DollsRef2`)) true false)
              (if (>= (`/Game/Blueprint/VoodooDolls/BP_Inventory.nbPuttingDolls` (`self.InventoryRef`)) 2)
                (`SceneComponent.SetVisibility` (`/Game/Blueprint/VoodooDolls/BP_VoodooDollsOnAutel.Cube` (`self.DollsRef3`)) true false)
                (if (>= (`/Game/Blueprint/VoodooDolls/BP_Inventory.nbPuttingDolls` (`self.InventoryRef`)) 3)
                  (`SceneComponent.SetVisibility` (`/Game/Blueprint/VoodooDolls/BP_VoodooDollsOnAutel.Cube` (`self.DollsRef4`)) true false)
                  (if (>= (`/Game/Blueprint/VoodooDolls/BP_Inventory.nbPuttingDolls` (`self.InventoryRef`)) 4)
                    (`SceneComponent.SetVisibility` (`/Game/Blueprint/VoodooDolls/BP_VoodooDollsOnAutel.Cube` (`self.DollsRef5`)) true false)
                    (`KismetSystemLibrary.Delay` 1.0)
                    (`/Game/Blueprint/Doors/BP_Door.openDoor` (`self.BPDoorRef`))))))))))
    (else
      (`KismetSystemLibrary.PrintString` "You don't have any doll" true true (struct :`R` 1.0 :`B` 0.050213 :`A` 1.0)))))

(fn `UserConstructionScript`)