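; BP_Teleport is a trigger volume that teleports the first-person character along world X when it overlaps the box.
; The new X comes from the TP variable's X, transformed by the actor's transform, while Y and Z keep the character movement's last update location.
; If the referenced closing Blueprint has ClosedOnce set, it also increments the NbTP teleport counter and prints debug messages.
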(event `self.Box.OnComponentBeginOverlap`
  (params (OverlappedComponent :type "PrimitiveComponent Object Reference") (OtherActor :type "Actor Object Reference") (OtherComp :type "PrimitiveComponent Object Reference") (OtherBodyIndex :type Integer) (bFromSweep :type Boolean) (SweepResult :type "HitResult Structure (by ref)"))
  (bind _tp_x (`KismetMathLibrary.BreakVector` (`self.TP`)))
  (bind _returnvalue_x (`KismetMathLibrary.BreakVector` (`KismetMathLibrary.TransformLocation` (`self.GetTransform`) (`KismetMathLibrary.Conv_DoubleToVector` _tp_x))))
  (bind _asbp_first_person_character (cast `/Game/FirstPerson/Blueprints/BP_FirstPersonCharacter` OtherActor))
  (bind (_returnvalue_x_2 _returnvalue_y _returnvalue_z) (`KismetMathLibrary.BreakVector` (`CharacterMovementComponent.GetLastUpdateLocation` (`Character.CharacterMovement` _asbp_first_person_character))))
  (`self.K2_SetActorLocation` _asbp_first_person_character (`KismetMathLibrary.MakeVector` _returnvalue_x _returnvalue_y _returnvalue_z) false false)
  (if (`/Game/Blueprint/BP_ClosingDoor.ClosedOnce` (`self.BPClosingRef`))
    (`KismetSystemLibrary.PrintString` "Yes close" true true (struct :`R` 1.0 :`G` 0.008642 :`A` 1.0))
    (bind _result (`/Engine/EditorBlueprintResources/StandardMacros.IncrementInt` (`self.nbTP`))
      (:`  `
        (bind _output_get (set `self.nbTP` _result))
        (`KismetSystemLibrary.PrintString` (`KismetStringLibrary.Conv_IntToString` _output_get) true true (struct :`R` 1.0 :`G` 0.008642 :`A` 1.0))))))

(fn `UserConstructionScript`)