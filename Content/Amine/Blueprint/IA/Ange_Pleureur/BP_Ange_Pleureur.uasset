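; BP_Ange_Pleureur is a Weeping Angel AI character that chases the player while unseen and freezes when watched.
; Each Tick, a dot product checks whether the angel is in the player's forward cone, then a camera-to-head-socket visibility trace checks for occlusion.
; It stops immediately if in view and unblocked, otherwise issues AIMoveTo toward the player.
; A separate Jetevois event calls PlayerNousVOis on its AIC_Ange controller.
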(event `self.ReceiveTick`
  (params (DeltaSeconds :type "Float (single-precision)"))
  (bind _returnvalue (`GameplayStatics.GetPlayerCharacter` 0))
  (if (> (`KismetMathLibrary.Dot_VectorVector` (`KismetMathLibrary.Normal` (- (`self.K2_GetActorLocation`) (`self.K2_GetActorLocation` _returnvalue))) (`self.GetActorForwardVector` _returnvalue)) 0.5)
    (bind (_outhit _returnvalue_2) (`KismetSystemLibrary.LineTraceSingle` (`self.K2_GetActorLocation` (`GameplayStatics.GetPlayerCameraManager` 0)) (`SceneComponent.GetSocketLocation` (`self.Mesh`) "head") "TraceTypeQuery1"))
    (if _returnvalue_2
      (`|AIMoveTo` self (0.0 0.0 0.0) (`GameplayStatics.GetPlayerCharacter` 0) :!label _label)
      (else
        (`MovementComponent.StopMovementImmediately` (`self.CharacterMovement`))))
    (else
      (goto _label))))

(event `/Game/Amine/Blueprint/IA/Ange_Pleureur/BPI_VoirMonstre.Jetevois`
  (bind _asaic_ange (cast `/Game/Amine/Blueprint/IA/Ange_Pleureur/AIC_Ange` (`AIBlueprintHelperLibrary.GetAIController` self)))
  (`/Game/Amine/Blueprint/IA/Ange_Pleureur/AIC_Ange.PlayerNousVOis` _asaic_ange))

(fn `UserConstructionScript`)