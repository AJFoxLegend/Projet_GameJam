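; BP_TPLevel is a teleport trigger that loads another level by name when its box is overlapped.
; The overlap only triggers travel once the inventory reference reports at least four placed dolls.
; It caches the first-person player character on BeginPlay and, if the flashlight is on, switches it off and waits briefly before opening the level.
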(event `self.ReceiveBeginPlay`
  (bind _asbp_first_person_character (cast `/Game/FirstPerson/Blueprints/BP_FirstPersonCharacter` (`GameplayStatics.GetPlayerCharacter` 0)))
  (set `self.Character_Ref` _asbp_first_person_character))

(event `self.Box.OnComponentBeginOverlap`
  (params (OverlappedComponent :type "PrimitiveComponent Object Reference") (OtherActor :type "Actor Object Reference") (OtherComp :type "PrimitiveComponent Object Reference") (OtherBodyIndex :type Integer) (bFromSweep :type Boolean) (SweepResult :type "HitResult Structure (by ref)"))
  (bind _character_ref (`self.Character_Ref`))
  (if (>= (`/Game/Blueprint/VoodooDolls/BP_Inventory.nbPuttingDolls` (`self.inventoryRef`)) 4)
    (`KismetSystemLibrary.PrintString` "TP")
    (if (`/Game/FirstPerson/Blueprints/BP_FirstPersonCharacter.isFlashOn` _character_ref)
      (`/Game/FirstPerson/Blueprints/BP_FirstPersonCharacter.LightOff` _character_ref)
      (`KismetSystemLibrary.Delay` 0.1)
      (`GameplayStatics.OpenLevel` (`self.LevelName`))
      (else
        (`GameplayStatics.OpenLevel` (`self.LevelName`))))))

(fn `UserConstructionScript`)