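; Trigger-box teleporter that moves the first-person player within the map or opens another level, with flashlight flicker to accompany jumps.
; On overlap, it either loads LevelName or takes the player's location, replacing flagged axes with the actor's position plus TP offset.
; If the linked closing door is interactive, tunnel-change mode adds a fixed X shift.
; Otherwise it teleports normally, optionally incrementing NbTP once that door has closed.
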(event `self.ReceiveBeginPlay`)

(event `self.Box.OnComponentBeginOverlap`
  (params (OverlappedComponent :type "PrimitiveComponent Object Reference") (OtherActor :type "Actor Object Reference") (OtherComp :type "PrimitiveComponent Object Reference") (OtherBodyIndex :type Integer) (bFromSweep :type Boolean) (SweepResult :type "HitResult Structure (by ref)"))
  ;[1 1 1] Téléporte le joueur
  (bind _asbp_first_person_character (cast `/Game/FirstPerson/Blueprints/BP_FirstPersonCharacter` (`GameplayStatics.GetPlayerCharacter` 0)))
  (set `self.CharacterRef` _asbp_first_person_character)
  (if (`self.bIsLevelChanging`)
    (`self.TPLevel`)
    (else
      (`|ExecutionSequence`
        (:`then_0`
          (`self.GetPlayerLocation`))
        (:`then_1`
          (`self.GetNewLocation`))
        (:`then_2`
          (if (and (`/Game/Blueprint/Doors/BP_ClosingDoor.isInteractive` (`self.closingDoorRef`)) (`self.isTunnelChanging`))
            (`self.TunnelChanging`)
            (else
              (`self.Teleportation`))))))))

(fn `GetNewLocation`
  (bind (_returnvalue_x _returnvalue_y _returnvalue_z) (`KismetMathLibrary.BreakVector` (`self.K2_GetActorLocation`)))
  (bind (_returnvalue_x_2 _returnvalue_y_2) (`KismetMathLibrary.BreakVector` (`self.K2_GetActorLocation`)))
  (bind _returnvalue_x_3 (`KismetMathLibrary.BreakVector` (`self.K2_GetActorLocation`)))
  (bind (_tp_x _tp_y) (`KismetMathLibrary.BreakVector` (`self.TP`)))
  (bind _tp_x_2 (`KismetMathLibrary.BreakVector` (`self.TP`)))
  (bind (_tp_x_3 _tp_y_2 _tp_z) (`KismetMathLibrary.BreakVector` (`self.TP`)))
  (bind _bismovinginy (`self.bIsMovingInY`))
  (bind _bismovinginz (`self.bIsMovingInZ`))
  (bind _bismovinginx (`self.bIsMovingInX`))
  (bind (_tempovector_x _tempovector_y) (`KismetMathLibrary.BreakVector` (`self.TempoVector`)))
  (bind (_tempovector_x_2 _tempovector_y_2 _tempovector_z) (`KismetMathLibrary.BreakVector` (`self.TempoVector`)))
  (bind (_tempovector_x_3 _tempovector_y_3 _tempovector_z_2) (`KismetMathLibrary.BreakVector` (`self.TempoVector`)))
  (`|ExecutionSequence`
    (:`then_0`
      (if _bismovinginx
        (bind _output_get (set `self.TempoVector` (`KismetMathLibrary.MakeVector` (+ _returnvalue_x_3 _tp_x_2) _tempovector_y_2 _tempovector_z)))
        (`KismetSystemLibrary.PrintString` (`KismetStringLibrary.Concat_StrStr` "2) On a is Moving X qui est  " (`KismetStringLibrary.Conv_BoolToString` _bismovinginx) " et tempo vector  " (`KismetStringLibrary.Conv_VectorToString` _output_get)) true true (struct :`R` 0.779096 :`G` 1.0 :`A` 1.0) 20.0)))
    (:`then_1`
      (if _bismovinginy
        (bind _output_get_2 (set `self.TempoVector` (`KismetMathLibrary.MakeVector` _tempovector_x_3 (+ _returnvalue_y_2 _tp_y) _tempovector_z_2)))
        (`KismetSystemLibrary.PrintString` (`KismetStringLibrary.Concat_StrStr` "2) On a is Moving Y qui est " (`KismetStringLibrary.Conv_BoolToString` _bismovinginy) " et tempo vector " (`KismetStringLibrary.Conv_VectorToString` _output_get_2)) true true (struct :`R` 0.779096 :`G` 1.0 :`A` 1.0) 20.0)))
    (:`then_2`
      (if _bismovinginz
        (bind _output_get_3 (set `self.TempoVector` (`KismetMathLibrary.MakeVector` _tempovector_x _tempovector_y (+ _returnvalue_z _tp_z))))
        (`KismetSystemLibrary.PrintString` (`KismetStringLibrary.Concat_StrStr` "2) On a is Moving Z qui est " (`KismetStringLibrary.Conv_BoolToString` _bismovinginz) " et tempo vector " (`KismetStringLibrary.Conv_VectorToString` _output_get_3)) true true (struct :`R` 0.779096 :`G` 1.0 :`A` 1.0) 20.0)))))

(fn `GetPlayerLocation`
  (bind _output_get (set `self.TempoVector` (`CharacterMovementComponent.GetLastUpdateLocation` (`Character.CharacterMovement` (`self.CharacterRef`)))))
  (`KismetSystemLibrary.PrintString` (`KismetStringLibrary.Concat_StrStr` "1) Player Location : " (`KismetStringLibrary.Conv_VectorToString` _output_get)) true true (struct :`R` 1.0 :`B` 0.057804 :`A` 1.0) 20.0))

(fn `Teleportation`
  (bind _characterref (`self.CharacterRef`))
  (bind _tempovector (`self.TempoVector`))
  (`SceneComponent.K2_SetWorldLocation` (`Actor.RootComponent` (`self.CharacterRef`)) _tempovector false false)
  (`KismetSystemLibrary.PrintString` (`KismetStringLibrary.Concat_StrStr` "On a le temp vector:" (`KismetStringLibrary.Conv_VectorToString` _tempovector) "actor location : ") true true (struct :`R` 0.320261 :`B` 1.0 :`A` 1.0) 20.0)
  (if (`self.bIsIncrementing`)
    (`/Game/FirstPerson/Blueprints/BP_FirstPersonCharacter.Light_Wink_TP` _characterref (`/Game/FirstPerson/Blueprints/BP_FirstPersonCharacter.isFlashOn` _characterref))
    (if (`/Game/Blueprint/Doors/BP_ClosingDoor.ClosedOnce` (`self.ClosingDoorRef`))
      (bind _result (`/Engine/EditorBlueprintResources/StandardMacros.IncrementInt` (`self.nbTP`))
        (:`  `
          (bind _output_get (set `self.nbTP` _result))
          (`KismetSystemLibrary.PrintString` (`KismetStringLibrary.Conv_IntToString` _output_get) true true (struct :`R` 1.0 :`G` 0.008642 :`A` 1.0)))))))

(fn `TPLevel`
  (bind _characterref (`self.CharacterRef`))
  (`KismetSystemLibrary.PrintString` "TP")
  (if (`/Game/FirstPerson/Blueprints/BP_FirstPersonCharacter.isFlashOn` (`self.CharacterRef`))
    (`/Game/FirstPerson/Blueprints/BP_FirstPersonCharacter.Light_Wink_TP` _characterref (`/Game/FirstPerson/Blueprints/BP_FirstPersonCharacter.isFlashOn` _characterref))
    (`/Game/FirstPerson/Blueprints/BP_FirstPersonCharacter.LightOff` (`self.CharacterRef`))
    (`GameplayStatics.OpenLevel` (`self.LevelName`))
    (else
      (`GameplayStatics.OpenLevel` (`self.LevelName`)))))

(fn `TunnelChanging`
  (bind _characterref (`self.CharacterRef`))
  (bind (_tempovector_x _tempovector_y _tempovector_z) (`KismetMathLibrary.BreakVector` (`self.TempoVector`)))
  (`SceneComponent.K2_SetWorldLocation` (`Actor.RootComponent` (`self.CharacterRef`)) (`KismetMathLibrary.MakeVector` (+ _tempovector_x 5507.0) _tempovector_y _tempovector_z) false false)
  (`/Game/FirstPerson/Blueprints/BP_FirstPersonCharacter.Light_Wink_TP` _characterref (`/Game/FirstPerson/Blueprints/BP_FirstPersonCharacter.isFlashOn` _characterref)))

(fn `UserConstructionScript`)