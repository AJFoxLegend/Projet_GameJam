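; BP_Door is a door actor that swings its static mesh around the yaw axis through open and close events.
; Each event plays its own timeline, whose RotationValue drives a Lerp every update.
; openDoor targets zero yaw and CloseDoor targets RotationAngle.
; Both blend from the mesh's current world yaw, re-read each update, and write the result as relative rotation.
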(event `openDoor`
  (bind (_returnvalue_roll _returnvalue_pitch _returnvalue_yaw) (`KismetMathLibrary.BreakRotator` (`SceneComponent.K2_GetComponentRotation` (`self.DoorStaticMeshComponent`))))
  (bind (_direction _rotationvalue) (`Timeline|Opening Door`)
    (:`Update`
      (`SceneComponent.K2_SetRelativeRotation` (`self.DoorStaticMeshComponent`) (`KismetMathLibrary.MakeRotator` 0.0 0.0 (`KismetMathLibrary.Lerp` _returnvalue_yaw 0.0 _rotationvalue)) false false))))

(event `CloseDoor`
  (bind (_returnvalue_roll _returnvalue_pitch _returnvalue_yaw) (`KismetMathLibrary.BreakRotator` (`SceneComponent.K2_GetComponentRotation` (`self.DoorStaticMeshComponent`))))
  (bind (_direction _rotationvalue) (`Timeline|Closing Door`)
    (:`Update`
      (`SceneComponent.K2_SetRelativeRotation` (`self.DoorStaticMeshComponent`) (`KismetMathLibrary.MakeRotator` 0.0 0.0 (`KismetMathLibrary.Lerp` _returnvalue_yaw (`self.rotationAngle`) _rotationvalue)) false false))))

(fn `UserConstructionScript`)