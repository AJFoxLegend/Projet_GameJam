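; Door actor Blueprint that swings its static mesh open and closed through openDoor and closeDoor events.
; Each event plays its own timeline, whose RotationValue track interpolates the mesh's relative yaw by RotationAngle in opposite directions.
; Opening and closing start from separate hardcoded base yaws rather than the current rotation, and neither timeline is reversed or restarted from the beginning.
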(event `openDoor`
  (bind (_direction _rotationvalue) (`Timeline|Opening Door`)
    (:`Update`
      (`SceneComponent.K2_SetRelativeRotation` (`self.DoorStaticMeshComponent`) (`KismetMathLibrary.MakeRotator` 0.0 0.0 (`KismetMathLibrary.Lerp` 90.0 (+ (* (`self.rotationAngle`) -1.0) 90.0) _rotationvalue)) false false))))

(event `closeDoor`
  (bind (_direction _rotationvalue) (`Timeline|Closing Door`)
    (:`Update`
      (`SceneComponent.K2_SetRelativeRotation` (`self.DoorStaticMeshComponent`) (`KismetMathLibrary.MakeRotator` 0.0 0.0 (`KismetMathLibrary.Lerp` 180.0 (+ (* (`self.rotationAngle`) 1.0) 180.0) _rotationvalue)) false false))))

(fn `UserConstructionScript`)